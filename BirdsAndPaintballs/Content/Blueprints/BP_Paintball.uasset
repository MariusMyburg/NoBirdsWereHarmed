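; BP_Paintball is a projectile actor for a paintball throw that lives for a few seconds.
; On BeginPlay it increments the throw counter on BP_GameMode and, when AttachCamera is set, switches the first player's view target to itself.
; Tick accumulates its age and destroys the actor once it passes a three-second lifetime.
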(event `self.ReceiveBeginPlay`
  (`|ExecutionSequence`
    (:`then_0`
      (bind _asbp_game_mode (cast `/Game/Blueprints/BP_GameMode` (`GameplayStatics.GetGameMode`)))
      (`/Engine/EditorBlueprintResources/StandardMacros.IncrementInt` (`/Game/Blueprints/BP_GameMode.NumBallsThrows` _asbp_game_mode)))
    (:`then_1`
      (if (`self.AttachCamera`)
        (`PlayerController.SetViewTargetWithBlend` (`GameplayStatics.GetPlayerController` 0) self 0.0 "VTBlend_Linear" 0.0 false)))))

(event `self.ReceiveTick`
  (params (DeltaSeconds :type "Float (single-precision)"))
  (set `self.Age` (+ DeltaSeconds (`self.Age`)))
  (if (> (`self.Age`) 3.0)
    (`self.K2_DestroyActor`)))

(fn `UserConstructionScript`)