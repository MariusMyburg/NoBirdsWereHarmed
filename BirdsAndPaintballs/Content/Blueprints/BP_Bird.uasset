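; Flying ibis target for a paintball game that registers itself with BP_GameMode on spawn and moves forward at a random speed, not scaled by delta time.
; Construction gives it a random material color and snaps the head collision sphere to the head socket.
; Paintball overlaps on head or body play different sounds, destroy the ball and call Hit, which increments the hit count, enables physics with physical animation and activates feathers.
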(event `self.ReceiveBeginPlay`
  (set `self.Speed` (`KismetMathLibrary.RandomFloatInRange` 3.0 8.0))
  (bind _asbp_game_mode (cast `/Game/Blueprints/BP_GameMode` (`GameplayStatics.GetGameMode`)))
  (`/Engine/EditorBlueprintResources/StandardMacros.IncrementInt` (`/Game/Blueprints/BP_GameMode.NumTargersSpawned` _asbp_game_mode)))

(event `self.ReceiveTick`
  (params (DeltaSeconds :type "Float (single-precision)"))
  (`self.K2_AddActorWorldOffset` (* (`self.GetActorForwardVector`) (`self.Speed`))))

(event `self.BodyCollisionCapsule.OnComponentBeginOverlap`
  (params (OverlappedComponent :type "PrimitiveComponent Object Reference") (OtherActor :type "Actor Object Reference") (OtherComp :type "PrimitiveComponent Object Reference") (OtherBodyIndex :type Integer) (bFromSweep :type Boolean) (SweepResult :type "HitResult Structure (by ref)"))
  (bind _asbp_paintball (cast `/Game/Blueprints/BP_Paintball` OtherActor))
  (`GameplayStatics.PlaySoundAtLocation` "/Game/Sounds/birds004.birds004" (`SceneComponent.K2_GetComponentLocation` (`self.SkeletalMesh`)))
  (`self.Hit`)
  (`self.K2_DestroyActor` _asbp_paintball))

(event `self.HeadCollisionSphere.OnComponentBeginOverlap`
  (params (OverlappedComponent :type "PrimitiveComponent Object Reference") (OtherActor :type "Actor Object Reference") (OtherComp :type "PrimitiveComponent Object Reference") (OtherBodyIndex :type Integer) (bFromSweep :type Boolean) (SweepResult :type "HitResult Structure (by ref)"))
  (bind _asbp_paintball (cast `/Game/Blueprints/BP_Paintball` OtherActor))
  (`GameplayStatics.PlaySoundAtLocation` "/Game/Sounds/birds003.birds003" (`SceneComponent.K2_GetComponentLocation` (`self.SkeletalMesh`)))
  (`self.Hit`)
  (`self.K2_DestroyActor` _asbp_paintball))

(fn `Hit`
  (bind _asbp_game_mode (cast `/Game/Blueprints/BP_GameMode` (`GameplayStatics.GetGameMode`)))
  (`/Engine/EditorBlueprintResources/StandardMacros.IncrementInt` (`/Game/Blueprints/BP_GameMode.NumTargetsHit` _asbp_game_mode)
    (:`  `
      (`PrimitiveComponent.SetSimulatePhysics` (`self.SkeletalMesh`) true)
      (`PhysicalAnimationComponent.SetSkeletalMeshComponent` (`self.PhysicalAnimation`) (`self.SkeletalMesh`))
      (`PhysicalAnimationComponent.ApplyPhysicalAnimationSettings` (`self.PhysicalAnimation`) "RootBone" (`self.PhysicalAnimationData`))
      (`ActorComponent.Activate` (`self.Feathers`) false))))

(fn `UserConstructionScript`
  (bind _returnvalue (`PrimitiveComponent.CreateDynamicMaterialInstance` (`self.SkeletalMesh`) 0 "/Game/Materials/MAT_Ibis_Inst.MAT_Ibis_Inst"))
  (`MaterialInstanceDynamic.SetVectorParameterValue` _returnvalue "Color" (`KismetMathLibrary.Conv_VectorToLinearColor` (* (`KismetMathLibrary.RandomUnitVector`) 200.0)))
  (`SceneComponent.K2_AttachToComponent` (`self.HeadCollisionSphere`) (`self.SkeletalMesh`) "HeadSocket" "SnapToTarget" "SnapToTarget" "KeepRelative" true))