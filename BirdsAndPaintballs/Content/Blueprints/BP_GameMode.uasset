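; Game mode that nags the player with a buy-full-version prompt every ten minutes of wall-clock time.
; Tick compares Now against the last show time, then creates the BP_BuyFullVersion widget, pauses the game and resets the timestamp.
; Unconnected leftover nodes hold a test HTTP GET request, its completion logging, an unpause and a device ID printout, none of which run.
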(event `self.ReceiveBeginPlay`
  (set `self.BuyPromptLastShowTime` (`KismetMathLibrary.Now`)))

(event `self.ReceiveTick`
  (params (DeltaSeconds :type "Float (single-precision)"))
  (if (> (`KismetMathLibrary.GetTotalMinutes` (- (`KismetMathLibrary.Now`) (`self.BuyPromptLastShowTime`))) 10.0)
    (bind _returnvalue (`|CreateWidget` "/Game/Blueprints/UMG/BP_BuyFullVersion.BP_BuyFullVersion_C" (`GameplayStatics.GetPlayerController` 0)))
    (`GameplayStatics.SetGamePaused` true)
    (`UserWidget.AddToViewport` _returnvalue 0)
    (set `self.BuyPromptLastShowTime` (`KismetMathLibrary.Now`))))

(event `OnRequestFailed`
  (params (Request :type "VaRestRequestJSON Object Reference"))
  (`KismetSystemLibrary.PrintString` "Request Failed"))

(event `OnRequestComplete`
  (params (Request :type "VaRestRequestJSON Object Reference")))

(fn `UserConstructionScript`)